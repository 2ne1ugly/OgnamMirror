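; A destructible actor that breaks apart through a physics field when its health runs out or three seconds after play begins.
; AnyDamage lowers Health to a floor of zero and calls Destruct at zero, while OnReset restores base health and restarts the timed destruction.
; Destruct sets a flag, applies external cluster strain through a box falloff at DestructyField's transform, disables BlockyField collision and prints a debug string.
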(event Custom|Destruct
  (Variables|Default|SetDestructed true)
  (Class|FieldSystemComponent|ApplyPhysicsField (Variables|Default|GetField%20System) true "Field_ExternalClusterStrain" 0 (Field|SetBoxFalloff (Variables|Default|GetBoxFalloff) (Variables|Default|Getmagnitude) 0.0 1.0 0.0 (Transformation|GetWorldTransform (Variables|Default|GetDestructy%20Field)) "Field_FallOff_None"))
  (Collision|SetCollisionEnabled (Variables|Default|GetBlocky%20Field) "NoCollision")
  (Development|PrintString "Hello"))

(event EventBeginPlay
  (Variables|Default|SetHealth (Variables|Default|GetBase%20Health))
  (Utilities|FlowControl|Delay 3.0)
  (CallFunction|Destruct))

(event Collision|EventActorBeginOverlap
  (params (OtherActor :type Actor%20Object%20Reference)))

(event EventTick
  (params (DeltaSeconds :type Float%20%28single-precision%29)))

(event Game|Damage|EventAnyDamage
  (params (Damage :type Float%20%28single-precision%29) (DamageType :type Damage%20Type%20Object%20Reference) (InstigatedBy :type Controller%20Object%20Reference) (DamageCauser :type Actor%20Object%20Reference))
  (bind _output_get (Variables|Default|SetHealth (Math|Float|Max(Float) (- (Variables|Default|GetHealth) Damage) 0.0)))
  (if (<= _output_get 0.0)
    (CallFunction|Destruct)))

(event EventOnReset
  (Variables|Default|SetHealth (Variables|Default|GetBase%20Health))
  (Utilities|FlowControl|Delay 3.0)
  (CallFunction|Destruct))

(fn ConstructionScript)