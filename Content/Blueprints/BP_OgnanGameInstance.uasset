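; BP_OgnanGameInstance is the Game Instance Blueprint, which reports network and travel failures as debug messages.
; It handles the network error and travel error events by formatting the failure type as text and printing it with Print String.
; The network message also includes the IsServer flag as an integer, and neither handler attempts any recovery.
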(event EventHandleNetworkError
  (params (FailureType :type ENetworkFailure%20Enum :default "NetDriverAlreadyExists") (bIsServer :type Boolean))
  (Development|PrintString (Utilities|String|ToString(Text) (Utilities|Text|FormatText "Network Error {s}:{E}" (Math|Conversions|ToInteger(Boolean) bIsServer) (Utilities|Text|ToText(String) (Utilities|String|EnumtoString FailureType))))))

(event EventHandleTravelError
  (params (FailureType :type ETravelFailure%20Enum :default "NoLevel"))
  (Development|PrintString (Utilities|String|ToString(Text) (Utilities|Text|FormatText "Travel Error:{E}" (Utilities|Text|ToText(String) (Utilities|String|EnumtoString FailureType))))))