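; OgnamUtils is a small set of utility functions for working with Text values.
; Each function converts the Text to a String first: TextSub returns a substring as Text, and ToInt parses an integer.
; TextIsNumeric also treats empty text as numeric.
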(fn TextSub
  (params (Source%20Text :type Text) (Start%20Index :type Integer) (Length :type Integer))
  (return (Utilities|Text|ToText(String) (Utilities|String|GetSubstring (Utilities|String|ToString(Text) Source%20Text) Start%20Index Length))))

(fn ToInt
  (params (Input%20Text :type Text))
  (return (Math|Conversions|ToInteger(Byte) (Utilities|String|ToString(Text) Input%20Text))))

(fn TextIsNumeric
  (params (Intput%20Text :type Text))
  (bind _returnvalue (Utilities|String|ToString(Text) Intput%20Text))
  (return (or (Class|KismetStringLibrary|IsNumeric _returnvalue) (== (Utilities|String|Len _returnvalue) 0))))